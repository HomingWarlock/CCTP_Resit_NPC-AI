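; BP_MovePoint is a world-space move point marker with a spinning floor/floating point visual and a camera-facing UI.
; On BeginPlay it finds actors implementing Int_Camera and uses the camera position they return to yaw the Scene component toward it.
; MovePointObjects spins on yaw, with both rotations driven by looping zero-delay macros instead of Tick.
; CancelledState swaps the FloorPoint and FloatingPoint materials to show cancellation.
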(event Custom|HandleUIRotation
  ;[0.7084 0 1 1 35] Handle UI Rotation
  (bind _outactors (Actor|GetAllActorswithInterface "/Game/MyAssets/Interfaces/RemakeThese/Player/Camera/Int_Camera.Int_Camera_C"))
  (for _array_element _outactors
    (Variables|Default|Setcam_ref _array_element)
    (Utilities|LoopForever(RotateUI))))

(event Custom|HandleRotation
  ;[1 0 0 1 35] Handle Rotation
  (Utilities|LoopForever(RotateObjects)))

(event Custom|CancelledState
  ;[1 0 0 1 35] Cancelled State
  (Rendering|Material|SetMaterial (Variables|Default|GetFloorPoint) 0 "/Game/MyAssets/Material/WorldUI/Markers/Mat_CancelledState.Mat_CancelledState")
  (Rendering|Material|SetMaterial (Variables|Default|GetFloatingPoint) 0 "/Game/MyAssets/Material/WorldUI/Markers/Mat_CancelledState.Mat_CancelledState"))

(event EventBeginPlay
  ;[0 0 1 1 35] Setup
  ;;[0 1 1 1 35] Trigger UI Rotate
  (CallFunction|HandleUIRotation)
  ;;[0 1 1 1 35] Trigger Object Rotate
  (CallFunction|HandleRotation))

(fn ConstructionScript)