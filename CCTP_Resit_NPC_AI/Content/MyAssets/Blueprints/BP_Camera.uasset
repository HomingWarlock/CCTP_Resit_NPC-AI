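; BP_Camera is a player-controlled camera pawn that moves, rotates and zooms through Enhanced Input.
; On BeginPlay it adds the camera-mode mapping context and seeds control rotation from the camera's world rotation before enabling pawn control rotation on the spring arm.
; Move and ascend/descend actions drive movement input along actor axes, while rotate feeds controller yaw and pitch.
; Zoom adjusts camera field of view within clamped limits.
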(event Input|EnhancedActionEvents|EnhancedInputActionIA_Move
  (params (ActionValue :type Vector%202D%20Structure) (ElapsedSeconds :type Float%20%28double-precision%29) (TriggeredSeconds :type Float%20%28double-precision%29) (InputAction :type Input%20Action%20Object%20Reference :default "/Game/MyAssets/Input/CameraMode_Actions/IA_Move.IA_Move"))
  ;[0 0 1 1 35] X/Y Movement
  (Pawn|Input|AddMovementInput (Math|Vector|GetRightVector (Transformation|GetActorRotation)) (.x ActionValue) false)
  (Pawn|Input|AddMovementInput (Math|Vector|GetForwardVector (Transformation|GetActorRotation)) (.y ActionValue) false))

(event Input|EnhancedActionEvents|EnhancedInputActionIA_Ascend_Descend
  (params (ActionValue :type Float%20%28double-precision%29) (ElapsedSeconds :type Float%20%28double-precision%29) (TriggeredSeconds :type Float%20%28double-precision%29) (InputAction :type Input%20Action%20Object%20Reference :default "/Game/MyAssets/Input/CameraMode_Actions/IA_Ascend_Descend.IA_Ascend_Descend"))
  ;[0 0 1 1 35] Z Movement
  (Pawn|Input|AddMovementInput (Math|Vector|GetUpVector (Transformation|GetActorRotation)) ActionValue false))

(event Input|EnhancedActionEvents|EnhancedInputActionIA_Zoom
  (params (ActionValue :type Float%20%28double-precision%29) (ElapsedSeconds :type Float%20%28double-precision%29) (TriggeredSeconds :type Float%20%28double-precision%29) (InputAction :type Input%20Action%20Object%20Reference :default "/Game/MyAssets/Input/CameraMode_Actions/IA_Zoom.IA_Zoom"))
  ;[0 0 1 1 35] Zoom
  (Camera|SetFieldOfView (Variables|Default|GetCamera) (Math|Float|Clamp(Float) (+ (* ActionValue -1e+01) (Variables|/Script/Engine.CameraComponent|GetFieldOfView (Variables|Default|GetCamera))) 1e+01 9e+01)))

(event Input|EnhancedActionEvents|EnhancedInputActionIA_Rotate
  (params (ActionValue :type Vector%202D%20Structure) (ElapsedSeconds :type Float%20%28double-precision%29) (TriggeredSeconds :type Float%20%28double-precision%29) (InputAction :type Input%20Action%20Object%20Reference :default "/Game/MyAssets/Input/CameraMode_Actions/IA_Rotate.IA_Rotate"))
  ;[0 0 1 1 35] Rotate
  (Pawn|Input|AddControllerYawInput (.x ActionValue))
  (Pawn|Input|AddControllerPitchInput (.y ActionValue)))

(event EventBeginPlay
  ;[0 0 1 1 35] Set Input Map
  (Input|AddMappingContext (PlayerController|LocalPlayerSubsystems|GetEnhancedInputLocalPlayerSubsystem (Game|GetPlayerController 0)) "/Game/MyAssets/Input/IMC_CameraMode.IMC_CameraMode" 0 "(bIgnoreAllPressedKeysUntilRelease=True,bForceImmediately=False,bNotifyUserSettings=False)")
  ;[0 0 1 1 35] Set Camera Rotation
  (Pawn|SetControlRotation (Pawn|GetController) (Transformation|GetWorldRotation (Variables|Default|GetCamera)))
  (Variables|/Script/Engine.SpringArmComponent|SetbUsePawnControlRotation (Variables|Default|GetSpringArm) true))

(fn ConstructionScript)