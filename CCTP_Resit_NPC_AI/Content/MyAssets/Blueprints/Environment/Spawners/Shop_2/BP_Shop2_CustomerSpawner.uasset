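; Spawner actor for Shop 2 that creates AI_Shop2_Customer actors at the shop's true entrance point.
; It looks up the BP_Shop2_MapPoints actor in the level and spawns at its PointTrueEntrance location.
; One customer spawns on BeginPlay, and the CustomerSpawnerSpawn custom event repeats the same lookup and spawn whenever it is called.
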(event EventBeginPlay
  (bind _returnvalue (Actor|GetActorOfClass "/Game/MyAssets/Blueprints/Environment/MapPoints/Shop_2/BP_Shop2_MapPoints.BP_Shop2_MapPoints_C"))
  (bind _output_get (Variables|Default|SetMapPoints _returnvalue))
  (Game|SpawnActorfromClass "/Game/MyAssets/Blueprints/AI/2_Shop/Part2/Customer/AI_Shop2_Customer.AI_Shop2_Customer_C" (Math|Conversions|ToTransform(Vector) (Variables|/Game/MyAssets/Blueprints/Environment/MapPoints/Shop_2/BP_Shop2_MapPoints.BP_Shop2_MapPoints_C|GetPoint_TrueEntrance _output_get)) "Undefined" "MultiplyWithRoot" 0 0))

(event EventCustomerSpawnerSpawn
  (bind _returnvalue (Actor|GetActorOfClass "/Game/MyAssets/Blueprints/Environment/MapPoints/Shop_2/BP_Shop2_MapPoints.BP_Shop2_MapPoints_C"))
  (bind _output_get (Variables|Default|SetMapPoints _returnvalue))
  (Game|SpawnActorfromClass "/Game/MyAssets/Blueprints/AI/2_Shop/Part2/Customer/AI_Shop2_Customer.AI_Shop2_Customer_C" (Math|Conversions|ToTransform(Vector) (Variables|/Game/MyAssets/Blueprints/Environment/MapPoints/Shop_2/BP_Shop2_MapPoints.BP_Shop2_MapPoints_C|GetPoint_TrueEntrance _output_get)) "Undefined" "MultiplyWithRoot" 0 0))

(fn ConstructionScript)