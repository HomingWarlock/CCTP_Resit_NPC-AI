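; Shop counter Blueprint that tracks the line of customers queuing at it.
; On BeginPlay it resets the queue count and sets the maximum to the last index of its queue points array.
; Add and remove events update the member list and adjust the count by one, without checking the limit.
; GetQueueInfo exposes the current count and maximum to callers.
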(event EventAddQueueMemeber
  (params (Member :type AI%20Shop%202%20Customer%20Object%20Reference))
  (Utilities|Array|Add (Variables|Default|GetQueueMembers) Member)
  (Variables|Default|SetQueueState (+ (Variables|Default|GetQueueState) 1)))

(event EventRemoveQueueMember
  (params (Member :type AI%20Shop%202%20Customer%20Object%20Reference))
  (Utilities|Array|RemoveItem (Variables|Default|GetQueueMembers) Member)
  (Variables|Default|SetQueueState (- (Variables|Default|GetQueueState) 1)))

(event EventBeginPlay
  (Variables|Default|SetQueueState 0)
  (Variables|Default|SetMaxQueue (- (Utilities|Array|Length (Variables|Default|GetPoints_CustomerQueue)) 1)))

(fn ConstructionScript)

(fn GetQueueInfo
  (return (Variables|Default|GetQueueState) (Variables|Default|GetMaxQueue)))