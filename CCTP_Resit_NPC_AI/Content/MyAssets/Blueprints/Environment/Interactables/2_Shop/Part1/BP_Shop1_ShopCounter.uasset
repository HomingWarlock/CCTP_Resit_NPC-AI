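; Shop counter interactable for the first shop that manages a line of customer queue spots.
; On BeginPlay it resets the queue state, caps it at three, and fills the queue point array with evenly spaced positions stepping back along world X from its root.
; UpdateQueue increments the state and loops over actors implementing an interface, with an empty loop body, while GetQueueInfo returns the state and maximum.
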(event EventUpdateQueue
  (Variables|Default|SetQueueState (+ 1 (Variables|Default|GetQueueState)))
  (bind _outactors (Actor|GetAllActorswithInterface 0))
  (for _array_element _outactors
    _))

(event EventBeginPlay
  (bind _self self)
  (bind _defaultsceneroot (Variables|Default|GetDefaultSceneRoot _self))
  (bind _returnvalue (Transformation|GetWorldLocation _defaultsceneroot))
  (Variables|Default|SetQueueState 0)
  (Variables|Default|SetMaxQueue 3)
  (for (_ _array_index) (Variables|Default|GetPoints_CustomerQueue)
    (Utilities|Array|SetArrayElem (Variables|Default|GetPoints_CustomerQueue) _array_index (Math|Vector|MakeVector (.x (- (Transformation|GetWorldLocation (Variables|Default|GetDefaultSceneRoot self)) (* (+ _array_index 1) 100))) (.y _returnvalue) (.z _returnvalue)))))

(fn ConstructionScript)

(fn GetQueueInfo
  (return (Variables|Default|GetQueueState) (Variables|Default|GetMaxQueue)))