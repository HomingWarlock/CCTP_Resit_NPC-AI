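; BP_ShopCounter is an interactable shop counter that holds the data for a queue and a shopkeeper position.
; The AddtoQueue event appends an actor to the QueueActors array, and the graph has no removal or movement logic.
; Getter functions expose the queued actors, the queue spots and the shopkeeper spot to other Blueprints.
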(event EventAddtoQueue
  (params (Actor%20To%20Add :type Actor%20Object%20Reference))
  (Utilities|Array|Add (Variables|Default|GetQueueActors) Actor%20To%20Add))

(fn ConstructionScript)

(fn GetQueueInfo
  (return (Variables|Default|GetQueueActors)))

(fn GetQueuePoints
  (return (Variables|Default|GetQueueSpots)))

(fn GetShopkeeperPoint
  (return (Variables|Default|GetShopKeeperSpot)))