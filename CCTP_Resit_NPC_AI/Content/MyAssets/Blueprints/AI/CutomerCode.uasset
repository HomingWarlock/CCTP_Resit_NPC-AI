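; Shop customer AI actor meant to enter a store, queue at the counter, buy and leave.
; Tick turns its Scene component toward the Int_Camera actor and interpolates pending body rotation.
; The purchase event flashes an action bubble and notifies shopkeepers through an interface; queue updates decrement its position.
; AIMoveTo steps, polling rotation macros and queue messaging are unwired, leaving BeginPlay and most movement events empty.
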(event Custom|Enter%20Queue
  ;[0 1 0 1 35] Enter Queue
)

(event Custom|RotateTowards%28Counter%29
  ;[0 1 0 1 35] Rotate Towards (Shop Counter)
)

(event Custom|ExamineQueue
  ;[0 1 0 1 35] Examine Queue
)

(event Custom|TrueLeave
  ;[0 1 0 1 35] True Leave
)

(event Custom|LeaveStore
  ;[0 1 0 1 35] Leave Store
)

(event Custom|EnterStop
  ;[0 1 0 1 35] Enter Stop
)

(event Custom|RotateTowards%28Exit%29
  ;[0 1 0 1 35] Rotate Towards (Shop Exit)
)

(event EventTick
  (params (DeltaSeconds :type Float%20%28single-precision%29))
  ;[0.7098 0 1 1 35] Action UI Face Camera
  (bind _outactors (Actor|GetAllActorswithInterface "/Game/MyAssets/Interfaces/RemakeThese/Player/Camera/Int_Camera.Int_Camera_C"))
  (for _array_element _outactors
    (bind _cam_worldloc (Class|IntCamera|CameraReference(Message) _array_element))
    (Transformation|SetWorldRotation (Variables|Default|GetScene) (Math|Rotator|FindLookatRotation (Transformation|GetWorldLocation (Variables|Default|GetScene)) _cam_worldloc) false false)
    ;[0 1 0 1 35] Handle Rotation
    (if (Variables|Default|GetIsRotating)
      (Transformation|SetActorRotation (Math|Interpolation|RInterpTo (Transformation|GetActorRotation) (Variables|Default|GetRotateTarget) (Utilities|Time|GetWorldDeltaSeconds) 1e+01))
      (if (== (Math|Float|Round (.yaw (Transformation|GetActorRotation))) (Math|Float|Round (.yaw (Variables|Default|GetRotateTarget))))
        (Variables|Default|SetIsRotating false)))))

(event EventCustomerQueueUpdate
  ;[0 1 0 1 35] Queue Update
  (bind _output_get (Variables|Default|SetQueuePos (- (Variables|Default|GetQueuePos) 1))))

(event EventCustomerHandlePurchase
  ;[0 1 0 1 35] Handle Purchase
  (Utilities|FlowControl|Delay 1.0)
  (Rendering|SetVisibility (Variables|Default|GetActionBubble) true false)
  (Utilities|FlowControl|Delay 1.0)
  (Rendering|SetVisibility (Variables|Default|GetActionBubble) false false)
  (bind _outactors (Actor|GetAllActorswithInterface "/Game/MyAssets/Interfaces/RemakeThese/Int_Shop2_ShopkeeperEvents.Int_Shop2_ShopkeeperEvents_C"))
  (for _array_element _outactors
    (Class|IntShop2ShopkeeperEvents|ShopKeeperEndPurchase(Message) _array_element)))

(event EventBeginPlay
  ;[0.7084 0 1 1 35] Setup
  ;;[0 0 0 1 35] Hide Action UI
)

(fn ConstructionScript)