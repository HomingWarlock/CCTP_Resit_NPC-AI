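; AI shopkeeper pawn that wanders the level, hiding its action bubble on BeginPlay and starting a patrol loop.
; Each leg picks a random navigable point within a large radius, spawns a BP_MovePoint marker there, moves to it, then destroys it and repeats on success.
; ChangeState interrupts patrol by cancelling and destroying the marker and setting a flag, which a polling WaitUntil macro watches to stop movement.
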(event Custom|ChoosePatrolPoint
  ;[0 1 0 1 35] Choose Patrol Point
  (Development|PrintString "Setting New Point")
  (bind _randomlocation (Class|NavigationSystemV1|GetRandomLocationinNavigableRadius (Transformation|GetActorLocation) 3e+04 0 0))
  (CallFunction|SpawnPatrolPoint _randomlocation)
  (Utilities|FlowControl|Delay 0.5)
  (CallFunction|MovetoPoint _randomlocation))

(event Custom|MoveToPoint
  (params (Point :type Vector))
  ;[0 1 0 1 35] Move To Point
  (AI|AIMoveTo self Point 0 5.0 false
    (:then
      (Development|PrintString "Moving To Point")
      (Utilities|WaitUntil(Condition) (Variables|Default|GetStateChanged)
        (:Finish%20Wait
          (Components|Movement|StopMovementImmediately (Variables|Character|GetCharacterMovement))
          (Development|PrintString "Interrupted " true true "(R=0.000000,G=0.660000,B=1.000000,A=1.000000)" 5.0))))
    (:OnSuccess
      (Actor|DestroyActor (Variables|Default|Getcurrent_point_object))
      (Utilities|FlowControl|Delay 1.0)
      (CallFunction|ChoosePatrolPoint))))

(event Custom|ChangeState
  ;[1 0 0 1 35] Change State
  (Variables|Default|SetStateChanged true)
  (Default|CancelledState (Variables|Default|Getcurrent_point_object))
  (Utilities|FlowControl|Delay 0.5)
  (Actor|DestroyActor (Variables|Default|Getcurrent_point_object)))

(event Custom|SpawnPatrolPoint
  (params (Point :type Vector))
  ;[0 1 0 1 35] Spawn Patrol Point
  (bind _returnvalue (Game|SpawnActorfromClass "/Game/MyAssets/Blueprints/WorldUI/Markers/BP_MovePoint.BP_MovePoint_C" (Math|Conversions|ToTransform(Vector) Point) "Undefined" "MultiplyWithRoot" 0 0))
  (Variables|Default|Setcurrent_point_object _returnvalue))

(event EventBeginPlay
  ;[0 0 1 1 35] Setup
  ;;[0 1 1 1 35] Hide Action UI
  (Rendering|SetVisibility (Variables|Default|GetActionBubble) false false)
  ;;[0 1 1 1 35] Trigger Patrol
  (CallFunction|ChoosePatrolPoint))

(fn ConstructionScript)